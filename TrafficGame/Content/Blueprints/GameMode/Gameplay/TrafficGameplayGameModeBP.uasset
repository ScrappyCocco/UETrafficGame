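; Game mode Blueprint for traffic gameplay that shows the start, next-round and end screens.
; Three events validate the supplied widget class, printing an error if it is invalid, then pass it to CreateAndShowWidget.
; That helper adds the widget to the viewport, switches to UI-only input focused on it and shows the cursor.
; Pressing Escape opens the main menu level.
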(event `Key|Escape`
  (params (Key :type "Key Structure"))
  ;[1 1 1] Back to Main Menu
  (:`Pressed`
    (`GameplayStatics.OpenLevelBySoftObjectPtr` "/Game/Maps/MainMenu/MainMenu.MainMenu")))

(event `self.ShowGameplayStartWidget`
  (params (Widget :type "UserWidget Class Reference"))
  ;[1 1 1] Pre Gameplay Widget
  (if (`KismetSystemLibrary.IsValidClass` Widget)
    (`self.CreateAndShowWidget` Widget)
    (else
      (`KismetSystemLibrary.PrintString` "Gameplay Start Widget Invalid!" true true (struct :`R` 1.0 :`A` 1.0) 5.0))))

(event `self.ShowNextRoundWidget`
  (params (Widget :type "UserWidget Class Reference"))
  ;[1 1 1] Next Round Widget
  (if (`KismetSystemLibrary.IsValidClass` Widget)
    (`self.CreateAndShowWidget` Widget)
    (else
      (`KismetSystemLibrary.PrintString` "Next Round Widget Invalid!" true true (struct :`R` 1.0 :`A` 1.0) 5.0))))

(event `self.ShowGameplayEndWidgetWidget`
  (params (Widget :type "UserWidget Class Reference"))
  ;[1 1 1] Post Gameplay Widget
  (if (`KismetSystemLibrary.IsValidClass` Widget)
    (`self.CreateAndShowWidget` Widget)
    (else
      (`KismetSystemLibrary.PrintString` "Gameplay Start Widget Invalid!" true true (struct :`R` 1.0 :`A` 1.0) 5.0))))

(fn `CreateAndShowWidget`
  (params (Widget :type "UserWidget Class Reference"))
  (bind _returnvalue (`GameplayStatics.GetPlayerController` 0))
  (bind _returnvalue_2 (`|CreateWidget` Widget _returnvalue))
  (`UserWidget.AddToViewport` _returnvalue_2 0)
  (`WidgetBlueprintLibrary.SetInputMode_UIOnlyEx` _returnvalue _returnvalue_2)
  (set `PlayerController.bShowMouseCursor` true _returnvalue))

(fn `UserConstructionScript`)