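; Startup game mode that shows a simple loading widget, handles first-boot graphics setup, then requests the MainMenu level through the game instance.
; On BeginPlay it checks a FirstBootFlagBP save to decide whether first-boot setup can be skipped.
; Otherwise it loads user settings, applies hardware benchmark results to scale quality, enables VSync by default and saves the completion flag.
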(event `self.ReceiveBeginPlay`
  ;[1 1 1] Create Loading Text
  (bind _returnvalue (`|CreateWidget` "/Game/Blueprints/UI/Loading/SimpleLoadingPageBP.SimpleLoadingPageBP_C" (`GameplayStatics.GetPlayerController` 0)))
  (`UserWidget.AddToViewport` _returnvalue 0)
  ;[1 1 1] Check if the First Boot save exist and that we completed it
  (bind _returnvalue_2 (`GameplayStatics.DoesSaveGameExist` (`self.FirstBootSaveName`)))
  (if _returnvalue_2
    (bind _returnvalue_3 (`GameplayStatics.LoadGameFromSlot` (`self.FirstBootSaveName`)))
    (bind (_asfirst_boot_flag_bp _bsuccess) (cast `/Game/Blueprints/Save/FirstBootFlagBP` _returnvalue_3 :!pure true))
    (if (and (`/Game/Blueprints/Save/FirstBootFlagBP.FirstBootCompleted` _asfirst_boot_flag_bp) _bsuccess)
      (`KismetSystemLibrary.PrintString` "Skip First Boot")
      (else
        (`KismetSystemLibrary.PrintString` "Execute First Boot" :!label _label)
        ;[1 1 1] Load User Settings and Run a benchmark to scale the game if needed
        (bind _returnvalue_4 (`GameUserSettings.GetGameUserSettings`))
        (`GameUserSettings.LoadSettings` _returnvalue_4 true)
        (`GameUserSettings.ValidateSettings` _returnvalue_4)
        (`GameUserSettings.RunHardwareBenchmark` _returnvalue_4 10 1.0 1.0)
        (`GameUserSettings.ApplyHardwareBenchmarkResults` _returnvalue_4)
        (`GameUserSettings.SetVSyncEnabled` _returnvalue_4 true) ; Enable VSync By Default
        (`GameUserSettings.ApplySettings` _returnvalue_4 true)
        ;[1 1 1] Save First Boot as completed
        (bind _returnvalue_5 (`GameplayStatics.CreateSaveGameObject` "/Game/Blueprints/Save/FirstBootFlagBP.FirstBootFlagBP_C"))
        (set `/Game/Blueprints/Save/FirstBootFlagBP.FirstBootCompleted` true _returnvalue_5)
        (`GameplayStatics.SaveGameToSlot` _returnvalue_5 (`self.FirstBootSaveName`))))
    (else
      (goto _label)))
  (`TrafficGameGameInstance.RequestLevelLoadByRef` (cast `/Game/Blueprints/GameInstance/TrafficGameGameInstanceBP` (`GameplayStatics.GetGameInstance`) :!pure true) "/Game/Maps/MainMenu/MainMenu.MainMenu"))

(fn `UserConstructionScript`)