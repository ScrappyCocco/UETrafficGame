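; Player controller for test-driving wheeled vehicles that shows a speed and gear HUD.
; On BeginPlay it creates the TestDriveVehicleUI widget with MPH disabled and adds it to the viewport.
; It caches the vehicle movement component from the controlled pawn, both on possess and at BeginPlay.
; Each Tick it passes that component's forward speed and current gear to the widget.
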(event `self.ReceivePossess`
  (params (PossessedPawn :type "Pawn Object Reference"))
  (bind _aswheeled_vehicle_pawn (cast `WheeledVehiclePawn` PossessedPawn))
  (set `self.Vehicle Movement Component` (`WheeledVehiclePawn.VehicleMovementComponent` _aswheeled_vehicle_pawn)))

(event `self.ReceiveBeginPlay`
  (`parent.ReceiveBeginPlay`)
  (bind _returnvalue (`|CreateWidget` "/Game/Blueprints/UI/Test/TestDriveVehicleUI.TestDriveVehicleUI_C" self))
  (bind _output_get (set `self.HUD` _returnvalue))
  (`UserWidget.AddToViewport` _output_get 0)
  (bind _aswheeled_vehicle_pawn (cast `WheeledVehiclePawn` (`self.K2_GetPawn`)))
  (set `self.Vehicle Movement Component` (`WheeledVehiclePawn.VehicleMovementComponent` _aswheeled_vehicle_pawn)))

(event `self.ReceiveTick`
  (params (DeltaSeconds :type "Float (single-precision)"))
  (`/Game/Blueprints/UI/Test/TestDriveVehicleUI.UpdateSpeed` (`self.HUD`) (`ChaosVehicleMovementComponent.GetForwardSpeed` (`self.Vehicle Movement Component`)))
  (`/Game/Blueprints/UI/Test/TestDriveVehicleUI.UpdateGear` (`self.HUD`) (`ChaosVehicleMovementComponent.GetCurrentGear` (`self.Vehicle Movement Component`))))

(fn `UserConstructionScript`)